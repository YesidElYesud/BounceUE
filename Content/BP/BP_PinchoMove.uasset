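; BP_PinchoMove is a moving thorn hazard that costs the player lives.
; Tick slides the thorn sprite between the first two spline points on a sine wave, with a random starting phase.
; Box overlap with a "Jugador"-tagged component adds points to BP_gi, then either respawns BP_Bola, deducting a life and refreshing its widget, or, below two lives, stores the level name and opens "Cargando".
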(event `self.ReceiveBeginPlay`
  (bind _asbp_gi (cast `/Game/BP/BP_gi` (`GameplayStatics.GetGameInstance`)))
  (set `self.As BP Gi` _asbp_gi)
  (set `self.Variancia` (`KismetMathLibrary.RandomFloatInRange` 0.0 3.0)))

(event `self.Box.OnComponentBeginOverlap`
  (params (OverlappedComponent :type "PrimitiveComponent Object Reference") (OtherActor :type "Actor Object Reference") (OtherComp :type "PrimitiveComponent Object Reference") (OtherBodyIndex :type Integer) (bFromSweep :type Boolean) (SweepResult :type "HitResult Structure (by ref)"))
  (bind _as_bp_gi (`self.As BP Gi`))
  (bind _as_bp_gi_2 (`self.As BP Gi`))
  (bind _as_bp_gi_3 (`self.As BP Gi`))
  (for _array_element (`ActorComponent.ComponentTags` OtherComp)
    (if (== _array_element "Jugador")
      (set `/Game/BP/BP_gi.Puntos` (+ (`/Game/BP/BP_gi.Puntos` _as_bp_gi) 5) _as_bp_gi)
      (if (> 2 (`/Game/BP/BP_gi.Vidas` _as_bp_gi_3))
        (bind _returnvalue (`GameplayStatics.GetCurrentLevelName` true))
        (set `/Game/BP/BP_gi.Nivel` (`KismetStringLibrary.Conv_StringToName` _returnvalue) _as_bp_gi_3)
        (`GameplayStatics.OpenLevel` "Cargando")
        (else
          (bind _asbp_bola (cast `/Game/BP/BP_Bola` OtherActor))
          (`self.K2_SetActorLocation` _asbp_bola (`/Game/BP/BP_gi.Vector Spawn` (`self.As BP Gi`)) false true)
          (set `/Game/BP/BP_gi.Vidas` (- (`/Game/BP/BP_gi.Vidas` _as_bp_gi_2) 1) _as_bp_gi_2)
          (`/Game/BP/BP_Bola.Actualizar WBP` _asbp_bola))))))

(event `self.ReceiveTick`
  (params (DeltaSeconds :type "Float (single-precision)"))
  (bind _spline (`self.Spline`))
  (bind _output_get (set `self.Variancia` (+ DeltaSeconds (`self.Variancia`))))
  (`SceneComponent.K2_SetRelativeLocation` (`self.dyn_thorn_2x_Sprite`) (`KismetMathLibrary.VLerp` (`.Position` (break `SplinePoint` (`SplineComponent.GetSplinePointAt` _spline 0 "Local"))) (`.Position` (break `SplinePoint` (`SplineComponent.GetSplinePointAt` _spline 1 "Local"))) (`KismetMathLibrary.MapRangeClamped` (`KismetMathLibrary.Sin` _output_get) 1.0 -1.0 1.0)) false false))

(fn `UserConstructionScript`)