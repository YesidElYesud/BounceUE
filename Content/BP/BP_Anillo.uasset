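; BP_Anillo is a ring that awards points the first time the player passes through it.
; On BeginPlay it increments the Anillos count in the BP_gi game instance.
; A box overlap with a component tagged "Jugador" fires once, adding to Puntos, darkening both ring sprites and decrementing Anillos.
; It then calls ActualizarWBP on the player's BP_Bola character, apparently to refresh the UI.
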(event `self.ReceiveBeginPlay`
  (bind _asbp_gi (cast `/Game/BP/BP_gi` (`GameplayStatics.GetGameInstance`)))
  (set `/Game/BP/BP_gi.Anillos` (+ (`/Game/BP/BP_gi.Anillos` _asbp_gi) 1) _asbp_gi)
  (set `self.As BP Gi` _asbp_gi))

(event `self.Box.OnComponentBeginOverlap`
  (params (OverlappedComponent :type "PrimitiveComponent Object Reference") (OtherActor :type "Actor Object Reference") (OtherComp :type "PrimitiveComponent Object Reference") (OtherBodyIndex :type Integer) (bFromSweep :type Boolean) (SweepResult :type "HitResult Structure (by ref)"))
  (bind _as_bp_gi (`self.As BP Gi`))
  (for _array_element (`ActorComponent.ComponentTags` OtherComp)
    (if (== _array_element "Jugador")
      (`/Engine/EditorBlueprintResources/StandardMacros.DoOnce` false
        (:`Completed`
          (set `/Game/BP/BP_gi.Puntos` (+ (`/Game/BP/BP_gi.Puntos` _as_bp_gi) 5) _as_bp_gi)
          (`PaperSpriteComponent.SetSpriteColor` (`self.ring_big_bottom_2x_Sprite`) (struct :`R` 0.026042 :`G` 0.026042 :`B` 0.026042 :`A` 1.0))
          (`PaperSpriteComponent.SetSpriteColor` (`self.ring_big_top_2x_Sprite`) (struct :`R` 0.026042 :`G` 0.026042 :`B` 0.026042 :`A` 1.0))
          (bind _asbp_gi (cast `/Game/BP/BP_gi` (`GameplayStatics.GetGameInstance`)))
          (set `/Game/BP/BP_gi.Anillos` (- (`/Game/BP/BP_gi.Anillos` _asbp_gi) 1) _asbp_gi)
          (bind _asbp_bola (cast `/Game/BP/BP_Bola` (`GameplayStatics.GetPlayerCharacter` 0)))
          (`/Game/BP/BP_Bola.Actualizar WBP` _asbp_bola))))))

(fn `UserConstructionScript`)