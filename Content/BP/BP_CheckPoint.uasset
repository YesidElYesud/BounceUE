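; BP_CheckPoint is a checkpoint actor that records its location as the player's spawn point.
; When its Sphere overlaps a component tagged "Jugador", a DoOnce gate lets it trigger a single time.
; It then writes its position to VectorSpawn in the BP_gi game instance, adds points to Puntos, swaps to the caught sprite and plays a sound.
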(event `self.Sphere.OnComponentBeginOverlap`
  (params (OverlappedComponent :type "PrimitiveComponent Object Reference") (OtherActor :type "Actor Object Reference") (OtherComp :type "PrimitiveComponent Object Reference") (OtherBodyIndex :type Integer) (bFromSweep :type Boolean) (SweepResult :type "HitResult Structure (by ref)"))
  (for _array_element (`ActorComponent.ComponentTags` OtherComp)
    (if (== _array_element "Jugador")
      (`/Engine/EditorBlueprintResources/StandardMacros.DoOnce` false
        (:`Completed`
          (bind _asbp_gi (cast `/Game/BP/BP_gi` (`GameplayStatics.GetGameInstance`)))
          (set `/Game/BP/BP_gi.Vector Spawn` (`self.K2_GetActorLocation`) _asbp_gi)
          (`PaperSpriteComponent.SetSprite` (`self.checkpoint_2x_Sprite`) "/Game/Imagenes/Sprites/checkpoint_catched_2x_Sprite.checkpoint_catched_2x_Sprite")
          (set `/Game/BP/BP_gi.Puntos` (+ (`/Game/BP/BP_gi.Puntos` _asbp_gi) 8) _asbp_gi)
          (`GameplayStatics.PlaySound2D` "/Game/Audio/MS_SFX_CheckPoint.MS_SFX_CheckPoint" 1.0 1.0 0.0 null null))))))

(fn `UserConstructionScript`)