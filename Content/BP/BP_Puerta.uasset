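; BP_Puerta is a level exit door that opens for the ball (BP_Bola) once the game instance's Anillos (rings) count is zero.
; The PFPortal flipbook starts stopped on its first frame; overlapping Box with zero rings disables its collision and plays it once.
; Overlapping Box1 with the ball loads the level named by LevelName, guarded by a DoOnce, without rechecking the ring count.
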(event `self.ReceiveBeginPlay`
  (bind _pf_portal (`self.PF_Portal`))
  (`PaperFlipbookComponent.Stop` _pf_portal)
  (`PaperFlipbookComponent.SetNewTime` _pf_portal 0.0)
  (bind _asbp_gi (cast `/Game/BP/BP_gi` (`GameplayStatics.GetGameInstance`)))
  (set `self.As BP Gi` _asbp_gi))

(event `self.Box.OnComponentBeginOverlap`
  (params (OverlappedComponent :type "PrimitiveComponent Object Reference") (OtherActor :type "Actor Object Reference") (OtherComp :type "PrimitiveComponent Object Reference") (OtherBodyIndex :type Integer) (bFromSweep :type Boolean) (SweepResult :type "HitResult Structure (by ref)"))
  (bind _pf_portal (`self.PF_Portal`))
  (cast `/Game/BP/BP_Bola` OtherActor)
  (if (== (`/Game/BP/BP_gi.Anillos` (`self.As BP Gi`)) 0)
    (`PrimitiveComponent.SetCollisionEnabled` (`self.PF_Portal`) "NoCollision")
    (`PaperFlipbookComponent.SetLooping` _pf_portal false)
    (`PaperFlipbookComponent.PlayFromStart` _pf_portal)))

(event `self.Box1.OnComponentBeginOverlap`
  (params (OverlappedComponent :type "PrimitiveComponent Object Reference") (OtherActor :type "Actor Object Reference") (OtherComp :type "PrimitiveComponent Object Reference") (OtherBodyIndex :type Integer) (bFromSweep :type Boolean) (SweepResult :type "HitResult Structure (by ref)"))
  (cast `/Game/BP/BP_Bola` OtherActor)
  (`/Engine/EditorBlueprintResources/StandardMacros.DoOnce` false
    (:`Completed`
      (`GameplayStatics.OpenLevel` (`self.Level Name`)))))

(fn `UserConstructionScript`)