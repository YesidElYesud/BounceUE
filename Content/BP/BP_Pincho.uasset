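; BP_Pincho is a spike hazard that penalizes the player on overlap with its box, detected by the "Jugador" component tag.
; Each hit adds points to the BP_gi game instance; with lives left, BP_Bola teleports to RefOrigen, loses a life and refreshes its widget.
; On the last life, it stores the current level name in the game instance and opens the "Cargando" level.
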(event `self.ReceiveBeginPlay`
  (bind _asbp_gi (cast `/Game/BP/BP_gi` (`GameplayStatics.GetGameInstance`)))
  (set `self.As BP Gi` _asbp_gi))

(event `self.Box.OnComponentBeginOverlap`
  (params (OverlappedComponent :type "PrimitiveComponent Object Reference") (OtherActor :type "Actor Object Reference") (OtherComp :type "PrimitiveComponent Object Reference") (OtherBodyIndex :type Integer) (bFromSweep :type Boolean) (SweepResult :type "HitResult Structure (by ref)"))
  (bind _as_bp_gi (`self.As BP Gi`))
  (bind _as_bp_gi_2 (`self.As BP Gi`))
  (bind _as_bp_gi_3 (`self.As BP Gi`))
  (for _array_element (`ActorComponent.ComponentTags` OtherComp)
    (if (== _array_element "Jugador")
      (set `/Game/BP/BP_gi.Puntos` (+ (`/Game/BP/BP_gi.Puntos` _as_bp_gi) 5) _as_bp_gi)
      (if (> 2 (`/Game/BP/BP_gi.Vidas` _as_bp_gi_3))
        (bind _returnvalue (`GameplayStatics.GetCurrentLevelName` true))
        (set `/Game/BP/BP_gi.Nivel` (`KismetStringLibrary.Conv_StringToName` _returnvalue) _as_bp_gi_3)
        (`GameplayStatics.OpenLevel` "Cargando")
        (else
          (bind _asbp_bola (cast `/Game/BP/BP_Bola` OtherActor))
          (`self.K2_SetActorLocation` _asbp_bola (`self.K2_GetActorLocation` (`self.Ref Origen`)) false true)
          (set `/Game/BP/BP_gi.Vidas` (- (`/Game/BP/BP_gi.Vidas` _as_bp_gi_2) 1) _as_bp_gi_2)
          (`/Game/BP/BP_Bola.Actualizar WBP` _asbp_bola))))))

(fn `UserConstructionScript`)